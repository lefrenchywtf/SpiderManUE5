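; BP_SMController is the player controller for the Spider-Man character.
; On BeginPlay it adds the IMC_SpiderMan Enhanced Input mapping context.
; Input actions for movement, look, jump and web swing are forwarded to the Chara reference, with web swing starting on press and stopping on release.
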(event `self.ReceiveBeginPlay`
  (`EnhancedInputSubsystemInterface.AddMappingContext` (subsystem `EnhancedInputLocalPlayerSubsystem`) "/Game/Core/Input/IMC_SpiderMan.IMC_SpiderMan" 0 (struct)))

(event `EnhancedInput|/Game/Core/Input/Actions/IA_Forward_Backward`
  (params (ActionValue :type "Float (double-precision)") (ElapsedSeconds :type "Float (double-precision)") (TriggeredSeconds :type "Float (double-precision)") (InputAction :type "InputAction Object Reference" :default "/Game/Core/Input/Actions/IA_Forward_Backward.IA_Forward_Backward"))
  (:`Triggered`
    (`/Game/Core/Blueprint/Character/BP_SMCharacter.MoveForward` (`self.Chara`) ActionValue)))

(event `EnhancedInput|/Game/Core/Input/Actions/IA_Left_Right`
  (params (ActionValue :type "Float (double-precision)") (ElapsedSeconds :type "Float (double-precision)") (TriggeredSeconds :type "Float (double-precision)") (InputAction :type "InputAction Object Reference" :default "/Game/Core/Input/Actions/IA_Left_Right.IA_Left_Right"))
  (:`Triggered`
    (`/Game/Core/Blueprint/Character/BP_SMCharacter.MoveSide` (`self.Chara`) ActionValue)))

(event `EnhancedInput|/Game/Core/Input/Actions/IA_Jump`
  (params (ActionValue :type Boolean) (ElapsedSeconds :type "Float (double-precision)") (TriggeredSeconds :type "Float (double-precision)") (InputAction :type "InputAction Object Reference" :default "/Game/Core/Input/Actions/IA_Jump.IA_Jump"))
  (:`Triggered`
    (`SMCharacter.JumpChara` (`self.Chara`))))

(event `EnhancedInput|/Game/Core/Input/Actions/IA_Look`
  (params (ActionValue :type "Vector2D Structure") (ElapsedSeconds :type "Float (double-precision)") (TriggeredSeconds :type "Float (double-precision)") (InputAction :type "InputAction Object Reference" :default "/Game/Core/Input/Actions/IA_Look.IA_Look"))
  (:`Triggered`
    (`SMCharacter.Look` (`self.Chara`) ActionValue)))

(event `EnhancedInput|/Game/Core/Input/Actions/IA_WebSwing`
  (params (ActionValue :type Boolean) (ElapsedSeconds :type "Float (double-precision)") (TriggeredSeconds :type "Float (double-precision)") (InputAction :type "InputAction Object Reference" :default "/Game/Core/Input/Actions/IA_WebSwing.IA_WebSwing"))
  (bind _chara (`self.Chara`))
  (:`Started`
    (`SMCharacter.StartWebswing` _chara))
  (:`Completed`
    (`SMCharacter.StopSwinging` _chara)))

(fn `UserConstructionScript`)